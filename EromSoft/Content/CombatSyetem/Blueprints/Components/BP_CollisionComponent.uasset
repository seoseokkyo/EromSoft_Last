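; Combat collision component that detects weapon, kick and pelvis-centered sphere hits.
; While each mode is enabled, Tick runs socket-based multi-sphere traces, using a shared already-hit list cleared on enable to report each actor once through CallOnHit.
; Weapon hits also destroy HiddenWall actors, and kicks turn victims to face the owner.
; It also toggles a Niagara weapon trail, positioned and sized from the weapon's start and end sockets.
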(event Custom|DisableTrailSystem
  ;[1 1 1] 무기 잔상 시스템
  ;;[1 1 1] DisableTrail
  (Components|Activation|Deactivate (Variables|Default|GetTrailEfecrVARIABLE)))

(event Custom|CollisionTrace
  (bind _collisionmeshcomponent (Variables|Default|GetCollisionMeshComponent))
  ;[1 1 1] CollisionTrace로 set hit.
  (bind _outhits (Collision|MultiSphereTraceForObjects (Transformation|GetSocketLocation _collisionmeshcomponent (Variables|Initialization|GetStart%20Socket%20Name)) (Transformation|GetSocketLocation _collisionmeshcomponent (Variables|Initialization|GetEnd%20Socket%20Name)) (Variables|Initialization|GetTrace%20Radius) (Variables|Initialization|GetCollision%20Object%20Types) false (Variables|Default|GetActors%20to%20Ignore) "None"))
  (for _array_element _outhits
    (bind _output_get (Variables|Default|SetLastHit _array_element))
    ;;[1 1 1] 이미 맞은애가 아니면 넘어가라
    (if (not (Utilities|Array|ContainsItem (Variables|Default|GetAlrreadyHitActors) (.HitActor (Collision|BreakHitResult _output_get))))
      (bind _output_get_2 (Variables|Default|SetHit%20Actor (.HitActor (Collision|BreakHitResult _output_get))))
      (Utilities|Array|Add (Variables|Default|GetAlrreadyHitActors) _output_get_2)
      (Default|CallOnHit (Variables|Default|GetLastHit)) ; 받는 애는 베이스 웨폰
      (bind _ashidden_wall (Utilities|Casting|CastToHiddenWall (Variables|Default|GetHit%20Actor)))
      (Default|DestroyEvent _ashidden_wall))))

(event Custom|EnableCollision
  ;[1 1 1] EnableCollision
  (CallFunction|ClearHitActors) ; 시작할 때 이미 맞은애 초기화
  (Variables|Default|SetbIsCollisionEnabled? true))

(event Custom|DisableCollision
  ;[1 1 1] DisableCollision
  (Variables|Default|SetbIsCollisionEnabled? false))

(event Custom|KickCollisionTrace
  (bind _collisionmeshcomponent (Variables|Default|GetCollisionMeshComponent))
  (bind _returnvalue (Transformation|GetSocketLocation _collisionmeshcomponent "KickEnd"))
  ;[1 1 1] CollisionTrace로 set hit.
  (bind _outhits (Collision|MultiSphereTraceForObjects (Transformation|GetSocketLocation _collisionmeshcomponent "KickStart") (Math|Vector|MakeVector (.x _returnvalue) (.y _returnvalue) (+ (.z _returnvalue) 2e+01)) (Variables|Default|GetKickRadius) (Variables|Initialization|GetCollision%20Object%20Types) false (Variables|Default|GetActors%20to%20Ignore) "None"))
  (for _array_element _outhits
    (bind _output_get (Variables|Default|SetLastHit _array_element))
    ;;[1 1 1] 이미 맞은애가 아니면 넘어가라
    (if (not (Utilities|Array|ContainsItem (Variables|Default|GetAlrreadyHitActors) (.HitActor (Collision|BreakHitResult _output_get))))
      (bind _output_get_2 (Variables|Default|SetHit%20Actor (.HitActor (Collision|BreakHitResult _output_get))))
      (Transformation|SetActorRotation _output_get_2 (Math|Rotator|MakeRotfromXZ (Math|Vector|Normalize (- (Transformation|GetActorLocation (Components|GetOwner)) (Transformation|GetActorLocation (.HitActor (Collision|BreakHitResult _output_get))))) (Transformation|GetActorUpVector (.HitActor (Collision|BreakHitResult _output_get)))) true)
      (Utilities|Array|Add (Variables|Default|GetAlrreadyHitActors) _output_get_2)
      (Default|CallOnHit (Variables|Default|GetLastHit)) ; 받는 애는 베이스 웨폰
    )))

(event Custom|Enable1
  ;[1 1 1] 원형 콜리전
  (CallFunction|ClearHitActors) ; 시작할 때 이미 맞은애 초기화
  (Variables|Default|SetbIsSphereCollisionEnabled? true))

(event Custom|SphereCollisionTrace
  (bind _collisionmeshcomponent (Variables|Default|GetCollisionMeshComponent))
  (bind _returnvalue (Transformation|GetSocketLocation _collisionmeshcomponent "PelvisSocket"))
  ;[1 1 1] CollisionTrace로 set hit.
  (bind _outhits (Collision|MultiSphereTraceForObjects (Transformation|GetSocketLocation _collisionmeshcomponent "PelvisSocket") (Math|Vector|MakeVector (.x _returnvalue) (.y _returnvalue) (+ (.z _returnvalue) 2e+01)) (Variables|Default|GetSphereRadius) (Variables|Initialization|GetCollision%20Object%20Types) false (Variables|Default|GetActors%20to%20Ignore) "None"))
  (for _array_element _outhits
    (bind _output_get (Variables|Default|SetLastHit _array_element))
    ;;[1 1 1] 이미 맞은애가 아니면 넘어가라
    (if (not (Utilities|Array|ContainsItem (Variables|Default|GetAlrreadyHitActors) (.HitActor (Collision|BreakHitResult _output_get))))
      (bind _output_get_2 (Variables|Default|SetHit%20Actor (.HitActor (Collision|BreakHitResult _output_get))))
      (Utilities|Array|Add (Variables|Default|GetAlrreadyHitActors) _output_get_2)
      (Default|CallOnHit (Variables|Default|GetLastHit)) ; 받는 애는 베이스 웨폰
    )))

(event Custom|Disable1
  ;[1 1 1] 원형 콜리전
  (Variables|Default|SetbIsSphereCollisionEnabled? false))

(event Custom|ClearHitActors
  ;[1 1 1] Call Hit Actor
  (Utilities|Array|Clear (Variables|Default|GetAlrreadyHitActors)))

(event Custom|SetCollisionMesh
  (params (MeshComponent :type Primitive%20Component%20Object%20Reference))
  ;[1 1 1] SetCollisionMeshComponent
  (Variables|Default|SetCollisionMeshComponent MeshComponent))

(event Custom|EnableKickCollision
  ;[1 1 1] Enable/Disable Kick Collision
  (CallFunction|ClearHitActors) ; 시작할 때 이미 맞은애 초기화
  (Variables|Default|SetbIsKickCollisionEnable? true))

(event Custom|DisableKickCollision
  ;[1 1 1] Enable/Disable Kick Collision
  (Variables|Default|SetbIsKickCollisionEnable? false))

(event Custom|EnableTrailSystem
  (bind _trailefecrvariable (Variables|Default|GetTrailEfecrVARIABLE))
  (bind _collisionmeshcomponent (Variables|Default|GetCollisionMeshComponent))
  (bind _start_socket_name (Variables|Initialization|GetStart%20Socket%20Name))
  (bind _end_socket_name (Variables|Initialization|GetEnd%20Socket%20Name))
  (bind _returnvalue (Transformation|GetSocketLocation _collisionmeshcomponent _start_socket_name))
  (bind _returnvalue_2 (Transformation|GetSocketLocation _collisionmeshcomponent _end_socket_name))
  ;[1 1 1] 무기 잔상 시스템
  ;;[1 1 1] EnableTrail
  (if true
    (Components|Activation|Activate _trailefecrvariable false)
    (Transformation|SetWorldLocation _trailefecrvariable (/ (+ _returnvalue _returnvalue_2) 2.0) false false)
    (Effects|Components|ParticleSystem|SetFloatParameter _trailefecrvariable "TrailWidth" (Math|Vector|VectorLength (- _returnvalue_2 _returnvalue)))))

(event EventTick
  (params (DeltaSeconds :type Float%20%28single-precision%29))
  (Utilities|FlowControl|Sequence
    (:then_0
      (if (Variables|Default|GetbIsCollisionEnabled?)
        (CallFunction|CollisionTrace)))
    (:then_1
      (if (Variables|Default|GetbIsKickCollisionEnable?)
        (CallFunction|KickCollisionTrace)))
    (:then_2
      (if (Variables|Default|GetbIsSphereCollisionEnabled?)
        (CallFunction|SphereCollisionTrace)))))

(fn GetAlreadyHitActors
  (return (Variables|Default|GetAlrreadyHitActors)))

(fn IsCollisionEnabled?
  (return (Variables|Default|GetbIsCollisionEnabled?)))

(fn GetLastHit
  (return (Variables|Default|GetLastHit)))

(fn GetColisionMeshComponent
  (return (Variables|Default|GetCollisionMeshComponent)))

(fn AddActortoIgnore
  (params (InActor :type Actor%20Object%20Reference%20%28by%20ref%29))
  (Utilities|Array|AddUnique (Variables|Default|GetActors%20to%20Ignore) InActor))

(fn RemoveAvtortoIgnore
  (params (InActorToRemove :type Actor%20Object%20Reference%20%28by%20ref%29))
  (Utilities|Array|RemoveItem (Variables|Default|GetActors%20to%20Ignore) InActorToRemove))

(fn GetActorstoIgnore
  (return (Variables|Default|GetActors%20to%20Ignore)))

(fn SetNaigaraSystemComp
  (params (NewParam :type Niagara%20Component%20Object%20Reference))
  (Variables|Default|SetTrailEfecrVARIABLE NewParam))