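; AI controller for the skeleton trap enemy BP_Skleton_Trap, driven by a state switch on Tick.
; Trap-type skeletons wait for an externally set target, then approach and kick once; others acquire the player within 800 units.
; It then chases and launches short attack combos separated by random cooldowns, returning home when the target strays too far from its origin.
; On death it stops, clears the target and unpossesses.
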(event Custom|Kick
  (bind _bp_skleton_trap (Variables|Default|GetBP_Skleton_Trap))
  (bind _combatcomponent (Variables|/Game/CombatSyetem/Blueprints/Enemy/Skeleton/BP_Skleton_Trap.BP_Skleton_Trap_C|GetCombatComponent _bp_skleton_trap))
  (if (Variables|/Game/CombatSyetem/Blueprints/Components/BP_CombatComponent.BP_CombatComponent_C|GetbIsAttacking _combatcomponent)
    (Variables|/Game/CombatSyetem/Blueprints/Components/BP_CombatComponent.BP_CombatComponent_C|SetbIsAttackSaved? _combatcomponent true)
    (else
      (Default|Kick _bp_skleton_trap)))
  (Variables|Default|SetOn%20Attack true)
  (Utilities|FlowControl|Delay 0.5)
  (Variables|Default|SetOn%20Attack false))

(event EventBeginPlay
  (CallFunction|InitCharacter))

(event EventTick
  (params (DeltaSeconds :type Float%20%28single-precision%29))
  (bind _returnvalue (Pawn|GetControlledPawn))
  (bind _bp_skleton_trap (Variables|Default|GetBP_Skleton_Trap))
  (bind _bp_skleton_trap_2 (Variables|Default|GetBP_Skleton_Trap))
  (bind _returnvalue_2 (Transformation|GetActorLocation _returnvalue))
  (bind _originlocation (Variables|/Game/CombatSyetem/Blueprints/Enemy/Skeleton/BP_Skleton_Trap.BP_Skleton_Trap_C|GetoriginLocation _bp_skleton_trap_2))
  (Utilities|IsValid (Pawn|GetControlledPawn)
    (:Is%20Valid
      (if (Utilities|Enum|NotEqual(Enum) (Variables|Default|GetcurrentState) "NewEnumerator5")
        (if (Variables|Default|GetenemyTrapType)
          (if (!= (Variables|Default|GetTarget) 0) :!label _label
            (Variables|Default|SetAttack%20Delay%20Time (+ DeltaSeconds (Variables|Default|GetAttack%20Delay%20Time)) :!label _label_2)
            (if (not (or (== (Variables|Default|GetCharacter%20Movement) 0) (== (Variables|Default|GetBP_Skleton_Trap) 0)))
              _
              (else
                (CallFunction|InitCharacter)))
            (switch Utilities|FlowControl|Switch|SwitchonBPE_ScketonEnum (Variables|Default|GetcurrentState)
              (:NewEnumerator0
                (Variables|Default|SetcurrentState "NewEnumerator1"))
              (:NewEnumerator1
                (if (>= (Math|Vector|Distance(Vector) (Transformation|GetActorLocation (Variables|Default|GetTarget)) (Variables|/Game/CombatSyetem/Blueprints/Enemy/Skeleton/BP_Skleton_Trap.BP_Skleton_Trap_C|GetoriginLocation (Variables|Default|GetBP_Skleton_Trap))) 1.2e+03)
                  (Variables|Default|SetcurrentState "NewEnumerator6")
                  (elif (>= (Variables|Default|GetAttack%20Delay%20Time) (Variables|Default|GetAttackDelayRand))
                    (if (<= (Utilities|GetPlayerDist) 2e+02)
                      (Variables|Default|SetcurrentState "NewEnumerator3")
                      (Variables|Default|SetAttack%20Delay%20Time 0.0)
                      (else
                        (CallFunction|MovetoPlayerFront :!label _label_3)))
                    (else
                      (goto _label_3)))))
              (:NewEnumerator2
                (if (Variables|Default|GetenemyTrapType)
                  (if (Variables|Default|GetTrapReacted)
                    (Variables|Default|SetcurrentState "NewEnumerator1" :!label _label_4)
                    (elif (<= (Math|Vector|Distance(Vector) (Transformation|GetActorLocation (Variables|Default|GetTarget)) (Transformation|GetActorLocation (Variables|Default|GetBP_Skleton_Trap))) 1.5e+02)
                      (CallFunction|Kick)
                      (Variables|Default|SetTrapReacted true)))
                  (else
                    (goto _label_4))))
              (:NewEnumerator3
                (if (<= (Variables|/Game/CombatSyetem/Blueprints/Enemy/Skeleton/BP_Skleton_Trap.BP_Skleton_Trap_C|GetcontinueAttackCount _bp_skleton_trap) 2)
                  (Default|Attack (Variables|Default|GetBP_Skleton_Trap))
                  (else
                    (Variables|Default|SetAttack%20Delay%20Time 0.0)
                    (Variables|/Game/CombatSyetem/Blueprints/Enemy/Skeleton/BP_Skleton_Trap.BP_Skleton_Trap_C|SetcontinueAttackCount _bp_skleton_trap 0)
                    (Variables|Default|SetcurrentState "NewEnumerator1")
                    (Variables|Default|SetAttackDelayRand (Math|Random|RandomFloatinRange 1.5 5.0)))))
              (:NewEnumerator5
                (CallFunction|Die))
              (:NewEnumerator6
                (if (<= (Math|Vector|Distance(Vector) (Math|Vector|MakeVector (.x _returnvalue_2) (.y _returnvalue_2) 0.0) (Math|Vector|MakeVector (.x _originlocation) (.y _originlocation) 0.0)) 5e+01)
                  (Transformation|SetActorLocation (Variables|Default|GetBP_Skleton_Trap) (Variables|/Game/CombatSyetem/Blueprints/Enemy/Skeleton/BP_Skleton_Trap.BP_Skleton_Trap_C|GetoriginLocation (Variables|Default|GetBP_Skleton_Trap)) false false)
                  (Variables|Default|SetcurrentState "NewEnumerator0")
                  (else
                    (AI|Navigation|MovetoLocation (Variables|/Game/CombatSyetem/Blueprints/Enemy/Skeleton/BP_Skleton_Trap.BP_Skleton_Trap_C|GetoriginLocation (Variables|Default|GetBP_Skleton_Trap)) 1e+01 true true false true 0))))))
          (elif (>= (Utilities|GetPlayerDist) 8e+02)
            (goto _label)
            (else
              (bind _asbp_combat_charactor (Utilities|Casting|CastToBP_CombatCharactor (Game|GetPlayerCharacter 0)))
              (if (!= (Variables|Default|GetTarget) 0)
                (goto _label)
                (else
                  (CallFunction|SetTragetPlayerGeneral _asbp_combat_charactor)
                  (goto _label_2))))))
        (else
          (CallFunction|Die))))))

(fn ConstructionScript)

(fn InitCharacter
  (Utilities|Casting|CastToCharacterMovementComponent (Pawn|GetMovementComponent (Pawn|GetControlledPawn)))
  (bind _asbp_skleton_trap (Utilities|Casting|CastToBP_Skleton_Trap (Pawn|GetControlledPawn)))
  (Variables|Default|SetBP_Skleton_Trap _asbp_skleton_trap))

(fn EnableAI
  (params (NewParam :type Boolean)))

(fn MovetoPlayerFront
  (Transformation|SetActorRotation (Pawn|GetControlledPawn) (Pawn|GetControlRotation :!class /Script/Engine.Controller))
  (AI|Navigation|MovetoActor (Game|GetPlayerCharacter 0) 1e+02 true true true "/Script/NavigationSystem.RecastFilter_UseDefaultArea")
  (return))

(fn RotatetoChr)

(fn InitCharacter
  (bind _asbp_skleton_trap (Utilities|Casting|CastToBP_Skleton_Trap (Pawn|GetControlledPawn)))
  (bind _output_get (Variables|Default|SetBP_Skleton_Trap _asbp_skleton_trap))
  (Variables|Default|SetenemyTrapType (Variables|/Game/CombatSyetem/Blueprints/Enemy/Skeleton/BP_Skleton_Trap.BP_Skleton_Trap_C|GetbTrapEnemy _output_get))
  (bind _output_get_2 (Variables|Default|SetCharacter%20Movement (Variables|/Script/Engine.Character|GetCharacterMovement _output_get)))
  (Variables|/Script/Engine.CharacterMovementComponent|SetMaxWalkSpeed _output_get_2 5e+02))

(fn SetTragetPlayerTrap
  (params (TargetPlayer :type BP%20Combat%20Charactor%20Object%20Reference))
  (bind _output_get (Variables|Default|SetTarget TargetPlayer))
  (Variables|Default|SetcurrentState "NewEnumerator2")
  (AI|SetFocus _output_get)
  (AI|Navigation|MovetoActor _output_get -1.0 true true true 0))

(fn SetTragetPlayerGeneral
  (params (TargetPlayer :type BP%20Combat%20Charactor%20Object%20Reference))
  (Variables|Default|SetTarget TargetPlayer))

(fn Die
  (Development|PrintString "Die")
  (AI|Navigation|StopMovement)
  (Variables|Default|SetTarget 0)
  (Pawn|UnPossess))