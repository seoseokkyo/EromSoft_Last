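; BP_Flower is the flower actor for Malenia's phase 2, an enemy effect built from three skeletal-mesh petals.
; OpenFlower starts all three petal montages together at a shared play rate.
; When the first petal's montage completes, the flower destroys itself and re-enables Malenia's AI.
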(event Custom|OpenFlower
  (Utilities|FlowControl|Sequence
    (:then_0
      (Animation|Montage|PlayMontage (Variables|Default|GetSkeletalMesh) "/Game/CombatSyetem/Blueprints/Enemy/Malenia/Phase2_Flower/Petal01_Anim_Montage.Petal01_Anim_Montage" (Variables|Default|GetplayLate)
        (:OnCompleted
          (Actor|DestroyActor)
          (Default|EnableAI (Variables|Default|GetmaleniaAI) true))))
    (:then_1
      (Animation|Montage|PlayMontage (Variables|Default|GetSkeletalMesh1) "/Game/CombatSyetem/Blueprints/Enemy/Malenia/Phase2_Flower/Petal02_Anim_Montage.Petal02_Anim_Montage" (Variables|Default|GetplayLate)))
    (:then_2
      (Animation|Montage|PlayMontage (Variables|Default|GetSkeletalMesh2) "/Game/CombatSyetem/Blueprints/Enemy/Malenia/Phase2_Flower/Petal03_Anim_Montage.Petal03_Anim_Montage" (Variables|Default|GetplayLate)))))

(event EventBeginPlay)

(event Collision|EventActorBeginOverlap
  (params (OtherActor :type Actor%20Object%20Reference)))

(event EventTick
  (params (DeltaSeconds :type Float%20%28single-precision%29)))

(fn ConstructionScript)