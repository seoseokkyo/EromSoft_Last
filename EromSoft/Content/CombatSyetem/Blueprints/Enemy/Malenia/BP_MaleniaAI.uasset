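; AI controller for the Malenia enemy, driving a BP_EnemyDoll1 pawn against the player once enabled.
; Tick runs an Idle/Move/Attack/Defensive state machine, lazily caching pawn and movement references.
; Move approaches or flanks by distance, then attacks when its timer allows or sidesteps to a randomly chosen, never-reset point.
; Attack picks close, middle or far moves by range, or buffers input mid-attack; the direction-randomizing collapsed graph is unconnected.
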(event Custom|EventSetIdle
  (Variables|Default|SetcurrentState "NewEnumerator0"))

(event EventBeginPlay)

(event EventTick
  (params (DeltaSeconds :type Float%20%28single-precision%29))
  (bind _returnvalue (Pawn|GetControlledPawn))
  (bind _as_bp_enemy_doll_1 (Variables|Default|GetAs%20BP%20Enemy%20Doll%201))
  (bind _as_bp_enemy_doll_1_2 (Variables|Default|GetAs%20BP%20Enemy%20Doll%201))
  (bind _as_bp_enemy_doll_1_3 (Variables|Default|GetAs%20BP%20Enemy%20Doll%201))
  (bind _returnvalue_2 (Transformation|GetActorRightVector _returnvalue))
  (bind _returnvalue_3 (Transformation|GetActorLocation _returnvalue))
  (bind _combatcomponent (Variables|/Game/CombatSyetem/Blueprints/BP_EnemyDoll1.BP_EnemyDoll1_C|GetCombatComponent _as_bp_enemy_doll_1))
  (bind _combatcomponent_2 (Variables|/Game/CombatSyetem/Blueprints/BP_EnemyDoll1.BP_EnemyDoll1_C|GetCombatComponent _as_bp_enemy_doll_1_2))
  (bind _combatcomponent_3 (Variables|/Game/CombatSyetem/Blueprints/BP_EnemyDoll1.BP_EnemyDoll1_C|GetCombatComponent _as_bp_enemy_doll_1_3))
  (if (Variables|Default|GetbEnableAI)
    (Variables|Default|SetAttackDelay%20Time (+ DeltaSeconds (Variables|Default|GetAttackDelay%20Time)))
    (Variables|Default|SetCloseDirSelDelayTime (+ DeltaSeconds (Variables|Default|GetCloseDirSelDelayTime)))
    (if (Utilities|IsValid (Variables|Default|GetAs%20Character%20Movement%20Component))
      (if (Default|CanPerformAttack? (Variables|Default|GetAs%20BP%20Enemy%20Doll%201))
        (switch Utilities|FlowControl|Switch|SwitchonBPE_MaleniaState (Variables|Default|GetcurrentState)
          (:NewEnumerator0
            (bind _asbp_combat_charactor (Utilities|Casting|CastToBP_CombatCharactor (Game|GetPlayerCharacter 0)))
            (Utilities|IsValid _asbp_combat_charactor
              (:Is%20Valid
                (Variables|Default|SetAs%20BP%20Combat%20Charactor _asbp_combat_charactor)
                (Variables|Default|SetcurrentState "NewEnumerator1"))))
          (:NewEnumerator1
            (if (>= (Utilities|GetPlayerDist) 2e+03)
              (Variables|/Script/Engine.CharacterMovementComponent|SetMaxWalkSpeed (Variables|Default|GetAs%20Character%20Movement%20Component) 6e+02)
              (CallFunction|MovetoPlayerFront)
              (elif (>= (Utilities|GetPlayerDist) 1e+03)
                (Variables|/Script/Engine.CharacterMovementComponent|SetMaxWalkSpeed (Variables|Default|GetAs%20Character%20Movement%20Component) 2e+02)
                (CallFunction|MovetoPlayerSide (Variables|Default|GetMoveDir))
                (elif (>= (Variables|Default|GetAttackDelay%20Time) 5.0)
                  (Variables|Default|SetcurrentState "NewEnumerator2")
                  (Variables|Default|SetAttackDelay%20Time 0.0)
                  (else
                    (Variables|Default|SetcurrentState "NewEnumerator4"))))))
          (:NewEnumerator2
            (if (>= (Utilities|GetPlayerDist) 1e+03)
              (Variables|Default|SetcurrentState "NewEnumerator0")
              (elif (>= (Utilities|GetPlayerDist) 7e+02)
                (if (Variables|/Game/CombatSyetem/Blueprints/Components/BP_CombatComponent.BP_CombatComponent_C|GetbIsAttacking _combatcomponent_2)
                  (Variables|/Game/CombatSyetem/Blueprints/Components/BP_CombatComponent.BP_CombatComponent_C|SetbIsAttackSaved? _combatcomponent_2 true)
                  (else
                    (Default|FarDistanceAttack _as_bp_enemy_doll_1_2)))
                (Variables|Default|SetOn%20Attack true)
                (Utilities|FlowControl|Delay 0.5)
                (Variables|Default|SetOn%20Attack false)
                (Variables|Default|SetcurrentState "NewEnumerator1")
                (elif (>= (Utilities|GetPlayerDist) 4e+02)
                  ;[1 1 1] 중거리 공격 추가 필요
                  (if (Variables|/Game/CombatSyetem/Blueprints/Components/BP_CombatComponent.BP_CombatComponent_C|GetbIsAttacking _combatcomponent_3)
                    (Variables|/Game/CombatSyetem/Blueprints/Components/BP_CombatComponent.BP_CombatComponent_C|SetbIsAttackSaved? _combatcomponent_3 true)
                    (else
                      (Default|MiddleDistanceAttack _as_bp_enemy_doll_1_3)))
                  (Variables|Default|SetOn%20Attack true)
                  (Utilities|FlowControl|Delay 0.5)
                  (Variables|Default|SetOn%20Attack false)
                  (Variables|Default|SetcurrentState "NewEnumerator1")
                  (else
                    ;[1 1 1] 근거리 공격
                    (if (Variables|/Game/CombatSyetem/Blueprints/Components/BP_CombatComponent.BP_CombatComponent_C|GetbIsAttacking _combatcomponent)
                      (Variables|/Game/CombatSyetem/Blueprints/Components/BP_CombatComponent.BP_CombatComponent_C|SetbIsAttackSaved? _combatcomponent true)
                      (else
                        (Default|CloseDistanceAttack _as_bp_enemy_doll_1)))
                    (Variables|Default|SetOn%20Attack true)
                    (Utilities|FlowControl|Delay 0.5)
                    (Variables|Default|SetOn%20Attack false)
                    (Variables|Default|SetcurrentState "NewEnumerator1"))))))
          (:NewEnumerator4
            (if (>= (Variables|Default|GetDeffensiveExcuteTime) 3.0)
              (Variables|Default|SetcurrentState "NewEnumerator0")
              (Variables|Default|SetDeffensiveExcuteTime 0.0)
              (else
                (Variables|Default|SetDeffensiveExcuteTime (+ (Utilities|Time|GetWorldDeltaSeconds) (Variables|Default|GetDeffensiveExcuteTime)))
                (if (Variables|Default|GetbDirSelected)
                  (Utilities|FocustoPlayer)
                  (AI|Navigation|MovetoLocation (Variables|Default|GetTargetLoc) -1.0 true true false true 0)
                  (else
                    (Variables|Default|SetbDirSelected true)
                    (bind _output_get (Variables|Default|SetbDirRight (Math|Random|RandomBool)))
                    (if _output_get
                      (Variables|Default|SetTargetLoc (+ _returnvalue_3 (* _returnvalue_2 5e+02)))
                      (else
                        (Variables|Default|SetTargetLoc (+ _returnvalue_3 (* _returnvalue_2 -5e+02))))))))))))
      (else
        (CallFunction|InitCharacter)))))

(fn ConstructionScript)

(fn EnableAI
  (params (Enable :type Boolean))
  (bind _output_get (Variables|Default|SetbEnableAI Enable))
  (Development|PrintString (Utilities|String|Append "Enable AI : " (Utilities|String|ToString(Boolean) _output_get))))

(fn MovetoPlayerFront
  (Transformation|SetActorRotation (Pawn|GetControlledPawn) (Pawn|GetControlRotation :!class /Script/Engine.Controller))
  (AI|Navigation|MovetoActor (Game|GetPlayerCharacter 0) 5e+02 true true true "/Script/NavigationSystem.RecastFilter_UseDefaultArea")
  (return))

(fn MovetoPlayerSide
  (params (Direction :type BPE_MaleniaMoveDirection%20Enum :default "NewEnumerator0"))
  (Utilities|FocustoPlayer)
  (switch Utilities|FlowControl|Switch|SwitchonBPE_MaleniaMoveDirection Direction
    (:NewEnumerator0
      (AI|Navigation|MovetoActor (Game|GetPlayerCharacter 0) 5e+02 true true true "/Script/NavigationSystem.RecastFilter_UseDefaultArea")
      (return))
    (:NewEnumerator1
      (AI|Navigation|SimpleMovetoLocation self (Utilities|GetPlayerDistLoc -5e+02))
      (return))
    (:NewEnumerator2
      (AI|Navigation|SimpleMovetoLocation self (Utilities|GetPlayerDistLoc 5e+02))
      (return))))

(fn InitCharacter
  (bind _ascharacter_movement_component (Utilities|Casting|CastToCharacterMovementComponent (Pawn|GetMovementComponent (Pawn|GetControlledPawn))))
  (Variables|Default|SetAs%20Character%20Movement%20Component _ascharacter_movement_component)
  (bind _asbp_enemy_doll_1 (Utilities|Casting|CastToBP_EnemyDoll1 (Pawn|GetControlledPawn)))
  (Variables|Default|SetAs%20BP%20Enemy%20Doll%201 _asbp_enemy_doll_1))