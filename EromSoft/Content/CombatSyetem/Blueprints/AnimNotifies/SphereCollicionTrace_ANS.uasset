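; An anim notify state that opens and closes the main weapon's collision window during an animation, named for sphere collision tracing.
; On begin and end it gets the BP_CombatComponent from the mesh owner, takes the main weapon, and calls Enable1 or Disable1 on its BPCollisionComponent.
; Only the mesh component is validity-checked; the combat component and weapon are used unchecked.
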(fn ReceivedNotifyBegin
  (params (MeshComp :type Skeletal%20Mesh%20Component%20Object%20Reference) (Animation :type Anim%20Sequence%20Base%20Object%20Reference) (TotalDuration :type Float%20%28single-precision%29) (EventReference :type Anim%20Notify%20Event%20Reference%20Structure%20%28by%20ref%29))
  (Utilities|IsValid MeshComp
    (:Is%20Valid
      (Default|Enable1 (Variables|/Game/CombatSyetem/Blueprints/Actors/BP_BaseWeapon.BP_BaseWeapon_C|GetBP_CollisionComponent (Default|GetMainWeapon (Actor|GetComponentbyClass (Components|GetOwner MeshComp) "/Game/CombatSyetem/Blueprints/Components/BP_CombatComponent.BP_CombatComponent_C"))))
      (return false))
    (:Is%20Not%20Valid
      (return false))))

(fn ReceivedNotifyEnd
  (params (MeshComp :type Skeletal%20Mesh%20Component%20Object%20Reference) (Animation :type Anim%20Sequence%20Base%20Object%20Reference) (EventReference :type Anim%20Notify%20Event%20Reference%20Structure%20%28by%20ref%29))
  (Utilities|IsValid MeshComp
    (:Is%20Valid
      (Default|Disable1 (Variables|/Game/CombatSyetem/Blueprints/Actors/BP_BaseWeapon.BP_BaseWeapon_C|GetBP_CollisionComponent (Default|GetMainWeapon (Actor|GetComponentbyClass (Components|GetOwner MeshComp) "/Game/CombatSyetem/Blueprints/Components/BP_CombatComponent.BP_CombatComponent_C"))))
      (return false))
    (:Is%20Not%20Valid
      (return false))))