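; Interactable Grace-style rest point that sends the player to another level.
; Its sphere overlap tells BP_CombatCharactor when it enters or leaves the Grace, and Interact calls OnRest on the character, then opens NewMap after a short delay.
; Tick spins and wobbles two meshes and bobs one of them with a sine-driven world offset.
; GetCamera and CameraChange are empty stubs.
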(event OnComponentBeginOverlap(Sphere)
  (params (OverlappedComponent :type Primitive%20Component%20Object%20Reference) (OtherActor :type Actor%20Object%20Reference) (OtherComp :type Primitive%20Component%20Object%20Reference) (OtherBodyIndex :type Integer) (bFromSweep :type Boolean) (SweepResult :type Hit%20Result%20Structure%20%28by%20ref%29))
  (bind _asbp_combat_charactor (Utilities|Casting|CastToBP_CombatCharactor OtherActor))
  (Default|EnterGrace _asbp_combat_charactor))

(event OnComponentEndOverlap(Sphere)
  (params (OverlappedComponent :type Primitive%20Component%20Object%20Reference) (OtherActor :type Actor%20Object%20Reference) (OtherComp :type Primitive%20Component%20Object%20Reference) (OtherBodyIndex :type Integer))
  (bind _asbp_combat_charactor (Utilities|Casting|CastToBP_CombatCharactor OtherActor))
  (Default|OutGrace _asbp_combat_charactor))

(event Custom|EventGetCamera
  (CallFunction|GetCamera))

(event EventBeginPlay
  (Transformation|AddWorldOffset (Variables|Default|GetSolid_03B3355B) (Math|Vector|MakeVector 0.0 0.0 (* (Math|Trig|Sin(Radians) (* (* (Utilities|Time|GetGameTimeinSeconds) 2.0) (Variables|Default|GetFloating%20Speed))) (Variables|Default|GetFloatingRange))) false false))

(event Collision|EventActorBeginOverlap
  (params (OtherActor :type Actor%20Object%20Reference)))

(event EventTick
  (params (DeltaSeconds :type Float%20%28single-precision%29))
  (bind _returnvalue (Utilities|Time|GetGameTimeinSeconds))
  (bind _solid_03b3355b (Variables|Default|GetSolid_03B3355B))
  (bind _returnvalue_2 (* _returnvalue 2.0))
  (bind _returnvalue_3 (Math|Trig|Sin(Radians) _returnvalue_2))
  (bind _returnvalue_4 (* _returnvalue_3 0.1))
  (bind _returnvalue_5 (Math|Rotator|MakeRotator _returnvalue_4 _returnvalue_4 1.0))
  (Transformation|AddRelativeRotation _solid_03b3355b _returnvalue_5 false false)
  (Transformation|AddRelativeRotation (Variables|Default|GetStaticMesh) (* _returnvalue_5 1.0) false false)
  (Transformation|AddWorldOffset _solid_03b3355b (Math|Vector|MakeVector 0.0 0.0 (* (Math|Trig|Sin(Radians) (* _returnvalue_2 (Variables|Default|GetFloating%20Speed))) (Variables|Default|GetFloatingRange))) false false))

(event EventInteract
  (params (caller :type Actor%20Object%20Reference))
  (bind _asbp_combat_charactor (Utilities|Casting|CastToBP_CombatCharactor caller))
  (Default|OnRest _asbp_combat_charactor)
  (Utilities|FlowControl|Delay 1.5)
  (Game|OpenLevel(byObjectReference) "/Game/Maps/NewMap.NewMap"))

(fn ConstructionScript)

(fn GetCamera
  (return 0))

(fn CameraChange
  (params (InputCamera :type Camera%20Actor%20Object%20Reference))
  (return 0))