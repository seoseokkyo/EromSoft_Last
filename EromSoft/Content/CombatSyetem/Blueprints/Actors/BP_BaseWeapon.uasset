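; BP_BaseWeapon is a base weapon actor for the combat system that attaches to its owning character and deals damage on hit.
; On equip it attaches to the hand or stowed socket by combat state, registers as main weapon, sends its combat type to the AnimInstance and configures its collision component.
; That component's hits apply point damage to actors able to receive it.
; An event switches the mesh to physics simulation.
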(event OnHit(BP_CollisionComponent)
  (params (HitResult :type Hit%20Result%20Structure))
  (bind _hitactor (Collision|BreakHitResult HitResult))
  (bind _retutnvalue (Class|CombatBPI|CanReciveDamage(Message) _hitactor))
  (if _retutnvalue
    (Game|Damage|ApplyPointDamage _hitactor (Variables|Default|GetDamage) (Transformation|GetActorForwardVector (Components|GetOwner)) HitResult (Game|GetInstigatorController) self)))

(event Custom|SimulateWeaponPhysics
  (bind _returnvalue (CallFunction|GetItemMesh))
  (Collision|SetCollisionProfileName _returnvalue "PhysicsActor" true :!class /Script/Engine.PrimitiveComponent)
  (Physics|SetSimulatePhysics _returnvalue true))

(event EventBeginPlay
  (|CallParentFunction) ; 지금 이 노드는 비활성 상태입니다. \n핀을 끌어서 다른 노드를 연결하면 활성화됩니다.
)

(event Collision|EventActorBeginOverlap
  (params (OtherActor :type Actor%20Object%20Reference))
  (|CallParentFunction OtherActor) ; 지금 이 노드는 비활성 상태입니다. \n핀을 끌어서 다른 노드를 연결하면 활성화됩니다.
)

(event EventTick
  (params (DeltaSeconds :type Float%20%28single-precision%29))
  (|CallParentFunction DeltaSeconds) ; 지금 이 노드는 비활성 상태입니다. \n핀을 끌어서 다른 노드를 연결하면 활성화됩니다.
)

(fn ConstructionScript
  (|CallParentFunction))

(fn OnEquipped
  ;[1 1 1] 무기 붙이고 메인 웨폰 설정
  (Variables|Default|SetCombatCombatComponent (Actor|GetComponentbyClass (Components|GetOwner) "/Game/CombatSyetem/Blueprints/Components/BP_CombatComponent.BP_CombatComponent_C"))
  (CallFunction|AttachActor (select (Default|IsCombatEnabled? (Variables|Default|GetCombatCombatComponent)) (Variables|초기화|GetHandSocketName) (Variables|Default|GetAttachSocket%20Name)))
  (Default|SetMainWeapon (Variables|Default|GetCombatCombatComponent) self)
  (Class|AnimInstanceBPI|UpdateCombatType(Message) (Components|SkeletalMesh|GetAnimInstance (Variables|/Script/Engine.Character|GetMesh (.AsCharacter (Utilities|Casting|CastToCharacter (Components|GetOwner))))) (Variables|초기화|GetCombatType))
  (Default|SetCollisionMesh (Variables|Default|GetBP_CollisionComponent) (CallFunction|GetItemMesh))
  (Default|AddActortoIgnore (Variables|Default|GetBP_CollisionComponent) (Components|GetOwner)))