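; FlotingThings is an actor that makes a static mesh bob vertically while its point light drifts around.
; BeginPlay randomizes a shared oscillation speed and a separate light multiplier for each axis.
; Tick applies a game-time sine wave as world offsets: Z only for the mesh, all three axes for the light.
; Offsets accumulate every frame without delta-time scaling, so travel distance depends on frame rate.
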(event EventBeginPlay
  (Variables|Default|SetSpeed (Math|Random|RandomFloatinRange 0.2 -0.2))
  (Variables|Default|SetSpeed_0 (Math|Random|RandomFloatinRange 2.0 -2.0))
  (Variables|Default|SetSpeed_1 (Math|Random|RandomFloatinRange 2.0 -2.0))
  (Variables|Default|SetSpeed_2 (Math|Random|RandomFloatinRange 2.0 -2.0)))

(event EventTick
  (params (DeltaSeconds :type Float%20%28single-precision%29))
  (bind _returnvalue (Utilities|Time|GetGameTimeinSeconds))
  (bind _speed (Variables|Default|GetSpeed))
  (bind _returnvalue_2 (* _returnvalue _speed))
  (bind _returnvalue_3 (Math|Trig|Sin(Radians) _returnvalue_2))
  (bind _returnvalue_4 (* _returnvalue_3 5.0))
  (bind _returnvalue_5 (* _returnvalue_4 0.05))
  (bind _returnvalue_6 (* _returnvalue_5 1e+01))
  (bind _returnvalue_7 (* _returnvalue_6 1e+01))
  (Transformation|AddWorldOffset (Variables|Default|GetStaticMesh) (Math|Vector|MakeVector 0.0 0.0 _returnvalue_6) false false)
  (Transformation|AddWorldOffset (Variables|Default|GetPointLight) (Math|Vector|MakeVector (* _returnvalue_7 (Variables|Default|GetSpeed_0)) (* _returnvalue_7 (Variables|Default|GetSpeed_1)) (* _returnvalue_7 (Variables|Default|GetSpeed_2))) false false))

(fn ConstructionScript)