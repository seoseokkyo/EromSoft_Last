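; BP_Message_Item is an interactable actor that shows and dismisses an on-screen message.
; Each Interact toggles the OnMessege flag, either creating a UI_Message4 widget and adding it to the viewport or removing it, with a 2D sound for each.
; MainChr movement is locked while the message is open and restored on close.
; An unconnected TrapKick call never runs.
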(event EventBeginPlay
  (|CallParentFunction) ; This node is disabled and will not be called.\nDrag off pins to build functionality.
)

(event Collision|EventActorBeginOverlap
  (params (OtherActor :type Actor%20Object%20Reference))
  (|CallParentFunction OtherActor) ; This node is disabled and will not be called.\nDrag off pins to build functionality.
)

(event EventTick
  (params (DeltaSeconds :type Float%20%28single-precision%29))
  (|CallParentFunction DeltaSeconds) ; This node is disabled and will not be called.\nDrag off pins to build functionality.
)

(event EventInteract
  (params (caller :type Actor%20Object%20Reference))
  (bind _mainchr (Variables|Default|GetMainChr))
  (if (Variables|Default|GetOnMessege?)
    (Audio|PlaySound2D "/Game/CombatSyetem/CourseFile/SoundFX/Menu/QuitSFX.QuitSFX" 3.0 1.0 0.0 0 0)
    (Variables|Default|SetOnMessege? false)
    (Widget|RemovefromParent (stale _returnvalue))
    (Default|CanMove _mainchr)
    (else
      (Audio|PlaySound2D "/Game/CombatSyetem/CourseFile/SoundFX/Menu/OpenMessageSFX.OpenMessageSFX" 3.0 1.0 0.0 0 0)
      (Variables|Default|SetOnMessege? true)
      (bind _returnvalue (UserInterface|CreateWidget "/Game/CombatSyetem/CourseFile/UI/UI_Message4.UI_Message4_C"))
      (UserInterface|Viewport|AddtoViewport _returnvalue 0)
      (Default|CantMove _mainchr))))

(fn ConstructionScript
  (|CallParentFunction))